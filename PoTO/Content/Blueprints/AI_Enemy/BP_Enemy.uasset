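; Enemy character Blueprint that chases the player on sight, takes hits and dies.
; Pawn sensing triggers AIMoveTo, and a detector overlap toggles the health bar widget for the player.
; OnHit plays a montage, subtracts Damage, updates the widget and destroys the actor near the death montage's end.
; Macros animate weapon draw/sheathe socket swaps and yaw turning toward an actor, though the turn call is unwired.
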(event OnSeePawn(PawnSensor)
  (params (Pawn :type Pawn%20Object%20Reference))
  ;[1 1 1] Enemy Follow Player
  (bind _asbp_base_character (Utilities|Casting|CastToBP_BaseCharacter Pawn))
  (AI|AIMoveTo self "0, 0, 0" _asbp_base_character 5.0 false))

(event OnComponentBeginOverlap(HealthBarDetector)
  (params (OverlappedComponent :type Primitive%20Component%20Object%20Reference) (OtherActor :type Actor%20Object%20Reference) (OtherComp :type Primitive%20Component%20Object%20Reference) (OtherBodyIndex :type Integer) (bFromSweep :type Boolean) (SweepResult :type Hit%20Result%20Structure%20%28by%20ref%29))
  ;[1 1 1] Health Bar Detector
  (Utilities|Casting|CastToBP_BaseCharacter OtherActor)
  (Rendering|SetVisibility (Variables|Default|GetHealthBar) true false))

(event OnComponentEndOverlap(HealthBarDetector)
  (params (OverlappedComponent :type Primitive%20Component%20Object%20Reference) (OtherActor :type Actor%20Object%20Reference) (OtherComp :type Primitive%20Component%20Object%20Reference) (OtherBodyIndex :type Integer))
  ;[1 1 1] Health Bar Detector
  (Utilities|Casting|CastToBP_BaseCharacter OtherActor)
  (Rendering|SetVisibility (Variables|Default|GetHealthBar) false false))

(event EventBeginPlay
  ;[1 1 1] Display Enemy Health Bar
  (bind _asbp_base_character (Utilities|Casting|CastToBP_BaseCharacter (Game|GetPlayerCharacter 0)))
  (Variables|Default|SetChar%20REF _asbp_base_character)
  (bind _asai_health_widget (Utilities|Casting|CastToAI_HealthWidget (UserInterface|GetUserWidgetObject (Variables|Default|GetHealthBar))))
  (Variables|Default|SetHealth%20Widget%20REF _asai_health_widget))

(event EventOnHit
  (params (Actor :type Actor%20Object%20Reference))
  ;[1 1 1] Enemy Hit and Death
  (bind _returnvalue (Animation|PlayAnimMontage "/Game/Animations/EnemyAI/EnemyHit_Montage.EnemyHit_Montage" 1.0 "None"))
  (bind _output_get (Variables|Default|SetHealth (- (Variables|Default|GetHealth) (Variables|Default|GetDamage))))
  (Variables|/Game/Blueprints/AI_Enemy/AI_HealthWidget.AI_HealthWidget_C|SetHealth (Variables|Default|GetHealth%20Widget%20REF) (Math|Conversions|ToFloat(Integer) _output_get))
  (if (<= _output_get 0)
    (bind _returnvalue_2 (Animation|PlayAnimMontage "/Game/Animations/EnemyAI/EnemyDeath_Montage.EnemyDeath_Montage" 1.0 "None"))
    (Utilities|FlowControl|Delay (- _returnvalue_2 0.3))
    (Actor|DestroyActor)))

(fn ConstructionScript)